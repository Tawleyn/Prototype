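; AI character Blueprint with a simple health pool and a combo melee attack.
; AnyDamage subtracts from CurrentHealth and prints the result; no death handling is present.
; MeleeAttack plays a montage and sphere-traces ahead, ignoring the player character, with explosion effects and sound at hits.
; A HasBeenHit flag limits damage to the first hit per swing, crediting the player controller as instigator, then breaks the loop.
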(event `self.ReceiveAnyDamage`
  (params (Damage :type "Float (single-precision)") (DamageType :type "DamageType Object Reference") (InstigatedBy :type "Controller Object Reference") (DamageCauser :type "Actor Object Reference"))
  (if true
    (bind _output_get (set `self.CurrentHealth` (- (`self.CurrentHealth`) Damage)))
    (`KismetSystemLibrary.PrintString` (`KismetStringLibrary.Concat_StrStr` "AI Health: " (`KismetStringLibrary.Conv_DoubleToString` _output_get)))))

(event `/Game/Characters/AI_Character/CombatInterface.MeleeAttack`
  (bind _returnvalue (`self.K2_GetActorLocation` self))
  (`|PlayMontage` (`self.Mesh`) "/Game/Characters/PlayerCharacter/Player_Character_Animations/Anims/SwordShield/Combo_1_Montage.Combo_1_Montage"
    (:`then`
      (bind _outhits (`KismetSystemLibrary.SphereTraceMulti` _returnvalue (+ _returnvalue (* (`self.GetActorForwardVector` self) 100.0)) 25.0 "TraceTypeQuery2" false (`|MakeArray` (`GameplayStatics.GetPlayerCharacter` 0) :!type "Actor Object Reference") "ForDuration"))
      (if true
        (for _array_element _outhits :!label _label
          (bind (_bblockinghit _binitialoverlap _time _distance _location _impactpoint _normal _impactnormal _physmat _hitactor) (`GameplayStatics.BreakHitResult` _array_element))
          (`GameplayStatics.SpawnEmitterAtLocation` "/Game/StarterContent/Particles/P_Explosion.P_Explosion" _impactpoint)
          (`GameplayStatics.PlaySoundAtLocation` "/Game/StarterContent/Audio/Explosion01.Explosion01" _impactpoint)
          (if (`self.HasBeenHit`)
            (`self.HitConfirmed`)
            (else
              (`GameplayStatics.ApplyDamage` _hitactor 35.0 (`GameplayStatics.GetPlayerController` 0) null "/Script/Engine.DamageType")
              (set `self.HasBeenHit` true))))
        (set `self.HasBeenHit` false)))))

(event `HitConfirmed`
  (goto _label :!via `Break`))

(fn `UserConstructionScript`)